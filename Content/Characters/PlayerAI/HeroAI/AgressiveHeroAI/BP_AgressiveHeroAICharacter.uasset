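; Aggressive hero AI character Blueprint that respawns itself after death instead of being destroyed.
; On BeginPlay it caches the location of the level's BP_SpawnPoint actor.
; DeathProcess flags the death, waits briefly, then calls SpawnHeroAI, which reuses the same actor.
; SpawnHeroAI teleless-moves it to a random reachable point around that spawn, resets ability system attributes, removes the Dead gameplay tag and clears the death flag.
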(event `self.ReceiveBeginPlay`
  (bind _returnvalue (`GameplayStatics.GetActorOfClass` "/Game/Shared/SpawnPoint/BP_SpawnPoint.BP_SpawnPoint_C"))
  (set `self.SpawnLocation` (`self.K2_GetActorLocation` _returnvalue)))

(event `Death Process`
  (set `self.IsDeath` true)
  (`KismetSystemLibrary.Delay` 0.2)
  (`self.SpawnHeroAI`))

(fn `SpawnHeroAI`
  (`self.K2_SetActorLocation` (`NavigationSystemV1.K2_GetRandomReachablePointInRadius` (`self.SpawnLocation`) 1260.0 null null))
  (`WarriorFunctionLibrary.ResetCharacterAttributes` (`self.WarriorAbilitySystemComponent`))
  (`WarriorFunctionLibrary.RemoveGameplayTagFromActorIfFound` self (struct :`TagName` "Shared.Status.Dead"))
  (set `self.IsDeath` false))

(fn `UserConstructionScript`)