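; Learning Agents interactor that defines observations and actions for the reinforcement-learning mutant monster boss, BP_MutantMonsterRL.
; Observes the boss's location and facing plus its NearestActor's location as "HeroAI", all relative to the boss's transform and only while that actor is valid.
; Writes rotation and X/Y movement float actions into ABP_MutantMonsterRL variables, clamping negative X to zero, so the animation Blueprint receives the policy output directly.
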(fn `GatherAgentObservation`
  (params (InObservationObject :type "LearningAgentsObservationObject Object Reference") (AgentId :type Integer))
  (returns (OutObservationObjectElement :type "LearningAgentsObservationObjectElement Structure"))
  (bind _obs_actor (`self.Obs Actor`))
  (bind _returnvalue (`Actor.GetTransform` _obs_actor))
  (bind _output_get (set `self.Obs Actor` (`self.GetAgent` AgentId "/Game/Characters/EnemyCharacter/MutantMonster/RLstuff/UEforum/BP_MutantMonsterRL.BP_MutantMonsterRL_C")))
  (`/Engine/EditorBlueprintResources/StandardMacros.IsValid` (`/Game/Characters/EnemyCharacter/MutantMonster/RLstuff/UEforum/BP_MutantMonsterRL.NearestActor` _output_get)
    (:`Is Valid`
      (return (`LearningAgentsObservations.MakeStructObservation` (`local.InObservationObject`) (`|MakeMap` "Boss" (`LearningAgentsObservations.MakeStructObservation` (`local.InObservationObject`) (`|MakeMap` "Location" (`LearningAgentsObservations.MakeLocationObservation` (`local.InObservationObject`) (`Actor.K2_GetActorLocation` _obs_actor) _returnvalue "LocationObservation" false null) "Direction" (`LearningAgentsObservations.MakeDirectionObservation` (`local.InObservationObject`) (`Actor.GetActorForwardVector` (`self.Obs Actor`)) _returnvalue "DirectionObservation" false null) :!type "Name")) "HeroAI" (`LearningAgentsObservations.MakeLocationObservation` (`local.InObservationObject`) (`Actor.K2_GetActorLocation` (`/Game/Characters/EnemyCharacter/MutantMonster/RLstuff/UEforum/BP_MutantMonsterRL.NearestActor` (`self.Obs Actor`))) (`Actor.GetTransform` (`self.Obs Actor`)) "LocationObservation" false null) :!type "Name"))))))

(fn `PerformAgentAction`
  (params (InActionObject :type "LearningAgentsActionObject Object Reference") (InActionObjectElement :type "LearningAgentsActionObjectElement Structure (by ref)") (AgentId :type Integer))
  (set `self.Act Actor` (`self.GetAgent` AgentId "/Game/Characters/EnemyCharacter/MutantMonster/RLstuff/UEforum/BP_MutantMonsterRL.BP_MutantMonsterRL_C"))
  (bind _outelements (`LearningAgentsActions.GetStructAction` (`local.InActionObject`) (`local.InActionObjectElement`)))
  (`|ExecutionSequence`
    (:`then_0`
      (bind _outvalue (`LearningAgentsActions.GetFloatAction` (`local.InActionObject`) (`BlueprintMapLibrary.Map_Find` _outelements "Rotation") "FloatAction" false null))
      (bind _asabp_mutant_monster_rl (cast `/Game/Characters/EnemyCharacter/MutantMonster/RLstuff/UEforum/AnimBP/ABP_MutantMonsterRL` (`SkeletalMeshComponent.GetAnimInstance` (`Character.Mesh` (`self.Act Actor`)))))
      (bind _output_get (set `self.As ABP Mutant Monster RL` _asabp_mutant_monster_rl))
      (set `/Game/Characters/EnemyCharacter/MutantMonster/RLstuff/UEforum/AnimBP/ABP_MutantMonsterRL.RotationYaw` _outvalue _output_get))
    (:`then_1`
      (bind _outelements_2 (`LearningAgentsActions.GetStructAction` (`local.InActionObject`) (`BlueprintMapLibrary.Map_Find` _outelements "Movement")))
      (`|ExecutionSequence`
        (:`then_0`
          (bind _outvalue_2 (`LearningAgentsActions.GetFloatAction` (`local.InActionObject`) (`BlueprintMapLibrary.Map_Find` _outelements_2 "XInput") "FloatAction" false null))
          (if (< _outvalue_2 0.0)
            (set `/Game/Characters/EnemyCharacter/MutantMonster/RLstuff/UEforum/AnimBP/ABP_MutantMonsterRL.MovementValueX` 0.0 (`self.As ABP Mutant Monster RL`))
            (else
              (set `/Game/Characters/EnemyCharacter/MutantMonster/RLstuff/UEforum/AnimBP/ABP_MutantMonsterRL.MovementValueX` _outvalue_2 (`self.As ABP Mutant Monster RL`)))))
        (:`then_1`
          (bind _outvalue_3 (`LearningAgentsActions.GetFloatAction` (`local.InActionObject`) (`BlueprintMapLibrary.Map_Find` _outelements_2 "YInput") "FloatAction" false null))
          (set `/Game/Characters/EnemyCharacter/MutantMonster/RLstuff/UEforum/AnimBP/ABP_MutantMonsterRL.MovementValueY` _outvalue_3 (`self.As ABP Mutant Monster RL`)))))))

(fn `Return Character Reference`)

(fn `SpecifyAgentAction`
  (params (InActionSchema :type "LearningAgentsActionSchema Object Reference"))
  (returns (OutActionSchemaElement :type "LearningAgentsActionSchemaElement Structure"))
  (return (`LearningAgentsActions.SpecifyStructAction` (`local.InActionSchema`) (`|MakeMap` "Rotation" (`LearningAgentsActions.SpecifyFloatAction` (`local.InActionSchema`)) "Movement" (`LearningAgentsActions.SpecifyStructAction` (`local.InActionSchema`) (`|MakeMap` "XInput" (`LearningAgentsActions.SpecifyFloatAction` (`local.InActionSchema`)) "YInput" (`LearningAgentsActions.SpecifyFloatAction` (`local.InActionSchema`)) :!type "Name")) :!type "Name"))))

(fn `SpecifyAgentObservation`
  (params (InObservationSchema :type "LearningAgentsObservationSchema Object Reference"))
  (returns (OutObservationSchemaElement :type "LearningAgentsObservationSchemaElement Structure"))
  (return (`LearningAgentsObservations.SpecifyStructObservation` (`local.InObservationSchema`) (`|MakeMap` "Boss" (`LearningAgentsObservations.SpecifyStructObservation` (`local.InObservationSchema`) (`|MakeMap` "Location" (`LearningAgentsObservations.SpecifyLocationObservation` (`local.InObservationSchema`)) "Direction" (`LearningAgentsObservations.SpecifyDirectionObservation` (`local.InObservationSchema`)) :!type "Name")) "HeroAI" (`LearningAgentsObservations.SpecifyLocationObservation` (`local.InObservationSchema`)) :!type "Name"))))