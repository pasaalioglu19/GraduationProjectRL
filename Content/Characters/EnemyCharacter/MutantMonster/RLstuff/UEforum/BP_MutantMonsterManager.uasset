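; Learning Agents manager that trains or runs neural-network control of mutant monsters.
; BeginPlay makes monsters tick after it, then builds interactor, policy, critic, training environment and shared-memory PPO trainer, even for inference.
; RunInference makes Tick run the policy instead of training, keeps saved network weights and resets monsters at start.
; Without it, networks reinitialize on every play.
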(event `self.ReceiveBeginPlay`
  (bind _shared_memory_settings (`self.Shared Memory Settings`))
  (bind _returnvalue (not (`self.RunInference`)))
  (`|ExecutionSequence`
    (:`then_0`
      (bind _outactors (`GameplayStatics.GetAllActorsOfClass` "/Game/Characters/EnemyCharacter/MutantMonster/RLstuff/UEforum/BP_MutantMonsterRL.BP_MutantMonsterRL_C"))
      (bind _output_get (set `self.Mutant Actors` _outactors))
      (`self.AddTickPrerequisiteActor` _output_get self))
    (:`then_1`
      (bind _returnvalue_2 (`LearningAgentsInteractor.MakeInteractor` (`self.LearningAgentsManager`) "/Game/Characters/EnemyCharacter/MutantMonster/RLstuff/UEforum/BP_MutantMonsterInteractor.BP_MutantMonsterInteractor_C" "MutantInteractor"))
      (set `self.Interactor` _returnvalue_2))
    (:`then_2`
      (bind _returnvalue_3 (`LearningAgentsPolicy.MakePolicy` (`self.LearningAgentsManager`) (`self.Interactor`) "/Script/LearningAgents.LearningAgentsPolicy" "MutantPolicy" "/Game/Characters/EnemyCharacter/MutantMonster/RLstuff/UEforum/DataAssets/DA_MutantNeuralNetworkEncoder.DA_MutantNeuralNetworkEncoder" "/Game/Characters/EnemyCharacter/MutantMonster/RLstuff/UEforum/DataAssets/DA_MutantNeuralNetworkPolicy.DA_MutantNeuralNetworkPolicy" "/Game/Characters/EnemyCharacter/MutantMonster/RLstuff/UEforum/DataAssets/DA_MutantNeuralNetworkDecoder.DA_MutantNeuralNetworkDecoder" _returnvalue _returnvalue _returnvalue (`self.Policy Settings`)))
      (set `self.Policy` _returnvalue_3))
    (:`then_3`
      (bind _returnvalue_4 (`LearningAgentsCritic.MakeCritic` (`self.LearningAgentsManager`) (`self.Interactor`) (`self.Policy`) "/Script/LearningAgents.LearningAgentsCritic" "MutantCritic" "/Game/Characters/EnemyCharacter/MutantMonster/RLstuff/UEforum/DataAssets/DA_MutantNeuralNetworkCritic.DA_MutantNeuralNetworkCritic" (not (`self.RunInference`)) (`self.Critic Settings`)))
      (set `self.Critic` _returnvalue_4))
    (:`then_4`
      (bind _returnvalue_5 (`LearningAgentsTrainingEnvironment.MakeTrainingEnvironment` (`self.LearningAgentsManager`) "/Game/Characters/EnemyCharacter/MutantMonster/RLstuff/UEforum/BP_MutantMonsterTrainingEnv.BP_MutantMonsterTrainingEnv_C"))
      (set `self.Training Env` _returnvalue_5))
    (:`then_5`
      (bind _returnvalue_6 (`LearningAgentsCommunicatorLibrary.SpawnSharedMemoryTrainingProcess` (`self.Trainer Process Settings`) _shared_memory_settings))
      (bind _returnvalue_7 (`LearningAgentsCommunicatorLibrary.MakeSharedMemoryCommunicator` _returnvalue_6 _shared_memory_settings))
      (set `self.Communicator` _returnvalue_7))
    (:`then_6`
      (bind _returnvalue_8 (`LearningAgentsPPOTrainer.MakePPOTrainer` (`self.LearningAgentsManager`) (`self.Interactor`) (`self.Training Env`) (`self.Policy`) (`self.Critic`) (`self.Communicator`) "/Script/LearningAgentsTraining.LearningAgentsPPOTrainer" "PPOTrainer" (`self.Trainer Settings`)))
      (set `self.PPOTrainer` _returnvalue_8))
    (:`then_7`
      (if (`self.RunInference`)
        (`/Game/Characters/EnemyCharacter/MutantMonster/RLstuff/UEforum/BP_MutantMonsterRL.Reset To Point` (`self.Mutant Actors`))
        (`KismetSystemLibrary.PrintString` "manager")))))

(event `self.ReceiveTick`
  (params (DeltaSeconds :type "Float (single-precision)"))
  (if (`self.RunInference`)
    (`LearningAgentsPolicy.RunInference` (`self.Policy`) 0.0)
    (else
      (`LearningAgentsPPOTrainer.RunTraining` (`self.PPOTrainer`) (`self.Trainer Training Settings`) (`self.Training Game Settings`) true true))))

(fn `UserConstructionScript`)