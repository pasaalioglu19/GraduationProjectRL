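; Learning Agents interactor that lets a reinforcement learning policy observe and control the Mutant Monster boss.
; Observations cover the boss and its nearest hero: location and direction relative to the boss, health ratio, boss ability flags and hero attack, block and roll states.
; Actions write rotation and movement to the AnimBP, zeroing negative X input, and set the ability float index and stop flag on the monster.
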(fn `GatherAgentObservation`
  (params (InObservationObject :type "LearningAgentsObservationObject Object Reference") (AgentId :type Integer))
  (returns (OutObservationObjectElement :type "LearningAgentsObservationObjectElement Structure"))
  (bind _obs_actor (`self.Obs Actor`))
  (bind _returnvalue (`Actor.GetTransform` _obs_actor))
  (bind _returnvalue_2 (`AbilitySystemBlueprintLibrary.GetAbilitySystemComponent` (`self.Obs Actor`)))
  (bind _returnvalue_3 (`Actor.GetTransform` (`self.Obs Actor`)))
  (bind _stopusingability (`/Game/Characters/EnemyCharacter/MutantMonster/RLstuff/UEforum/BP_MutantMonsterRL.StopUsingAbility` (`self.Obs Actor`)))
  (bind _isusingability2 (`/Game/Characters/EnemyCharacter/MutantMonster/RLstuff/UEforum/BP_MutantMonsterRL.IsUsingAbility2` (`self.Obs Actor`)))
  (bind _isusingability1 (`/Game/Characters/EnemyCharacter/MutantMonster/RLstuff/UEforum/BP_MutantMonsterRL.IsUsingAbility1` (`self.Obs Actor`)))
  (bind _isusingability3 (`/Game/Characters/EnemyCharacter/MutantMonster/RLstuff/UEforum/BP_MutantMonsterRL.IsUsingAbility3` (`self.Obs Actor`)))
  (bind _returnvalue_4 (`AbilitySystemBlueprintLibrary.GetAbilitySystemComponent` (`/Game/Characters/EnemyCharacter/MutantMonster/RLstuff/UEforum/BP_MutantMonsterRL.NearestActor` (`self.Obs Actor`))))
  (bind _output_get (set `self.Obs Actor` (`self.GetAgent` AgentId "/Game/Characters/EnemyCharacter/MutantMonster/RLstuff/UEforum/BP_MutantMonsterRL.BP_MutantMonsterRL_C")))
  (`/Engine/EditorBlueprintResources/StandardMacros.IsValid` (`/Game/Characters/EnemyCharacter/MutantMonster/RLstuff/UEforum/BP_MutantMonsterRL.NearestActor` _output_get)
    (:`Is Valid`
      (`KismetSystemLibrary.PrintString` null (`KismetStringLibrary.Concat_StrStr` "  B Ability 1 : " (`KismetStringLibrary.Conv_BoolToString` _isusingability1) "  B Ability 2 : " (`KismetStringLibrary.Conv_BoolToString` _isusingability2) "  B Ability 3 : " (`KismetStringLibrary.Conv_BoolToString` _isusingability3) "  B Stop Ability :  " (`KismetStringLibrary.Conv_BoolToString` _stopusingability)))
      (return (`LearningAgentsObservations.MakeStructObservation` (`local.InObservationObject`) (`|MakeMap` "Boss" (`LearningAgentsObservations.MakeStructObservation` (`local.InObservationObject`) (`|MakeMap` "Location" (`LearningAgentsObservations.MakeLocationObservation` (`local.InObservationObject`) (`Actor.K2_GetActorLocation` _obs_actor) _returnvalue "LocationObservation" false null) "Direction" (`LearningAgentsObservations.MakeDirectionObservation` (`local.InObservationObject`) (`Actor.GetActorForwardVector` (`self.Obs Actor`)) _returnvalue "DirectionObservation" false null) "Health" (`LearningAgentsObservations.MakeFloatObservation` (`local.InObservationObject`) (/ (`.ReturnValue` (`AbilitySystemComponent.GetGameplayAttributeValue` _returnvalue_2 (struct :`AttributeName` "CurrentHealth" :`Attribute` "/Script/GraduationProjectt.WarriorAttributeSet:CurrentHealth" :`AttributeOwner` "/Script/CoreUObject.Class'/Script/GraduationProjectt.WarriorAttributeSet'"))) (`.ReturnValue` (`AbilitySystemComponent.GetGameplayAttributeValue` _returnvalue_2 (struct :`AttributeName` "MaxHealth" :`Attribute` "/Script/GraduationProjectt.WarriorAttributeSet:MaxHealth" :`AttributeOwner` "/Script/CoreUObject.Class'/Script/GraduationProjectt.WarriorAttributeSet'")))) "FloatObservation" false null) "Ability" (`LearningAgentsObservations.MakeStructObservation` (`local.InObservationObject`) (`|MakeMap` "IsUsingAbility1" (`LearningAgentsObservations.MakeBoolObservation` (`local.InObservationObject`) _isusingability1 "BoolObservation" false null) "IsUsingAbility2" (`LearningAgentsObservations.MakeBoolObservation` (`local.InObservationObject`) _isusingability2 "BoolObservation" false null) "IsUsingAbility3" (`LearningAgentsObservations.MakeBoolObservation` (`local.InObservationObject`) _isusingability3 "BoolObservation" false null) "StopUsingAbility" (`LearningAgentsObservations.MakeBoolObservation` (`local.InObservationObject`) _stopusingability "BoolObservation" false null) :!type "Name")) :!type "Name")) "HeroAI" (`LearningAgentsObservations.MakeStructObservation` (`local.InObservationObject`) (`|MakeMap` "Location" (`LearningAgentsObservations.MakeLocationObservation` (`local.InObservationObject`) (`Actor.K2_GetActorLocation` (`/Game/Characters/EnemyCharacter/MutantMonster/RLstuff/UEforum/BP_MutantMonsterRL.NearestActor` (`self.Obs Actor`))) _returnvalue_3 "LocationObservation" false null) "Direction" (`LearningAgentsObservations.MakeDirectionObservation` (`local.InObservationObject`) (`Actor.GetActorForwardVector` (`/Game/Characters/EnemyCharacter/MutantMonster/RLstuff/UEforum/BP_MutantMonsterRL.NearestActor` (`self.Obs Actor`))) _returnvalue_3 "DirectionObservation" false null) "Health" (`LearningAgentsObservations.MakeFloatObservation` (`local.InObservationObject`) (/ (`.ReturnValue` (`AbilitySystemComponent.GetGameplayAttributeValue` _returnvalue_4 (struct :`AttributeName` "CurrentHealth" :`Attribute` "/Script/GraduationProjectt.WarriorAttributeSet:CurrentHealth" :`AttributeOwner` "/Script/CoreUObject.Class'/Script/GraduationProjectt.WarriorAttributeSet'"))) (`.ReturnValue` (`AbilitySystemComponent.GetGameplayAttributeValue` _returnvalue_4 (struct :`AttributeName` "MaxHealth" :`Attribute` "/Script/GraduationProjectt.WarriorAttributeSet:MaxHealth" :`AttributeOwner` "/Script/CoreUObject.Class'/Script/GraduationProjectt.WarriorAttributeSet'")))) "FloatObservation" false null) "State" (`LearningAgentsObservations.MakeStructObservation` (`local.InObservationObject`) (`|MakeMap` "IsAttacking" (`LearningAgentsObservations.MakeBoolObservation` (`local.InObservationObject`) (`/Game/Characters/PlayerAI/HeroAI/NormalHeroAI/BP_HeroAICharacter.IsAttacking` (`/Game/Characters/EnemyCharacter/MutantMonster/RLstuff/UEforum/BP_MutantMonsterRL.NearestActor` (`self.Obs Actor`))) "BoolObservation" false null) "IsBlocking" (`LearningAgentsObservations.MakeBoolObservation` (`local.InObservationObject`) (`/Game/Characters/PlayerAI/HeroAI/NormalHeroAI/BP_HeroAICharacter.IsBlocking` (`/Game/Characters/EnemyCharacter/MutantMonster/RLstuff/UEforum/BP_MutantMonsterRL.NearestActor` (`self.Obs Actor`))) "BoolObservation" false null) "IsRolling" (`LearningAgentsObservations.MakeBoolObservation` (`local.InObservationObject`) (`/Game/Characters/PlayerAI/HeroAI/NormalHeroAI/BP_HeroAICharacter.IsRolling` (`/Game/Characters/EnemyCharacter/MutantMonster/RLstuff/UEforum/BP_MutantMonsterRL.NearestActor` (`self.Obs Actor`))) "BoolObservation" false null) :!type "Name")) :!type "Name")) :!type "Name"))))))

(fn `PerformAgentAction`
  (params (InActionObject :type "LearningAgentsActionObject Object Reference") (InActionObjectElement :type "LearningAgentsActionObjectElement Structure (by ref)") (AgentId :type Integer))
  (set `self.Act Actor` (`self.GetAgent` AgentId "/Game/Characters/EnemyCharacter/MutantMonster/RLstuff/UEforum/BP_MutantMonsterRL.BP_MutantMonsterRL_C"))
  (bind _outelements (`LearningAgentsActions.GetStructAction` (`local.InActionObject`) (`local.InActionObjectElement`)))
  (`|ExecutionSequence`
    (:`then_0`
      (bind _outvalue (`LearningAgentsActions.GetFloatAction` (`local.InActionObject`) (`BlueprintMapLibrary.Map_Find` _outelements "Rotation") "FloatAction" false null))
      (bind _asabp_mutant_monster_rl (cast `/Game/Characters/EnemyCharacter/MutantMonster/RLstuff/UEforum/AnimBP/ABP_MutantMonsterRL` (`SkeletalMeshComponent.GetAnimInstance` (`Character.Mesh` (`self.Act Actor`)))))
      (bind _output_get (set `self.As ABP Mutant Monster RL` _asabp_mutant_monster_rl))
      (set `/Game/Characters/EnemyCharacter/MutantMonster/RLstuff/UEforum/AnimBP/ABP_MutantMonsterRL.RotationYaw` _outvalue _output_get))
    (:`then_1`
      (bind _outelements_2 (`LearningAgentsActions.GetStructAction` (`local.InActionObject`) (`BlueprintMapLibrary.Map_Find` _outelements "Movement")))
      (`|ExecutionSequence`
        (:`then_0`
          (bind _outvalue_2 (`LearningAgentsActions.GetFloatAction` (`local.InActionObject`) (`BlueprintMapLibrary.Map_Find` _outelements_2 "XInput") "FloatAction" false null))
          (if (< _outvalue_2 0.0)
            (set `/Game/Characters/EnemyCharacter/MutantMonster/RLstuff/UEforum/AnimBP/ABP_MutantMonsterRL.MovementValueX` 0.0 (`self.As ABP Mutant Monster RL`))
            (else
              (set `/Game/Characters/EnemyCharacter/MutantMonster/RLstuff/UEforum/AnimBP/ABP_MutantMonsterRL.MovementValueX` _outvalue_2 (`self.As ABP Mutant Monster RL`)))))
        (:`then_1`
          (bind _outvalue_3 (`LearningAgentsActions.GetFloatAction` (`local.InActionObject`) (`BlueprintMapLibrary.Map_Find` _outelements_2 "YInput") "FloatAction" false null))
          (set `/Game/Characters/EnemyCharacter/MutantMonster/RLstuff/UEforum/AnimBP/ABP_MutantMonsterRL.MovementValueY` _outvalue_3 (`self.As ABP Mutant Monster RL`)))))
    (:`then_2`
      (bind _outvalue_4 (`LearningAgentsActions.GetFloatAction` (`local.InActionObject`) (`BlueprintMapLibrary.Map_Find` _outelements "Ability") "FloatAction" false null))
      (set `/Game/Characters/EnemyCharacter/MutantMonster/RLstuff/UEforum/BP_MutantMonsterRL.UsingAbilityFloatIndex` _outvalue_4 (`self.Act Actor`)))
    (:`then_3`
      (bind _boutvalue (`LearningAgentsActions.GetBoolAction` (`local.InActionObject`) (`BlueprintMapLibrary.Map_Find` _outelements "Stop Ability") "BoolAction" false null))
      (set `/Game/Characters/EnemyCharacter/MutantMonster/RLstuff/UEforum/BP_MutantMonsterRL.StopUsingAbility` _boutvalue (`self.Act Actor`)))))

(fn `Return Character Reference`)

(fn `SpecifyAgentAction`
  (params (InActionSchema :type "LearningAgentsActionSchema Object Reference"))
  (returns (OutActionSchemaElement :type "LearningAgentsActionSchemaElement Structure"))
  (return (`LearningAgentsActions.SpecifyStructAction` (`local.InActionSchema`) (`|MakeMap` "Rotation" (`LearningAgentsActions.SpecifyFloatAction` (`local.InActionSchema`)) "Movement" (`LearningAgentsActions.SpecifyStructAction` (`local.InActionSchema`) (`|MakeMap` "XInput" (`LearningAgentsActions.SpecifyFloatAction` (`local.InActionSchema`)) "YInput" (`LearningAgentsActions.SpecifyFloatAction` (`local.InActionSchema`)) :!type "Name")) "Ability" (`LearningAgentsActions.SpecifyFloatAction` (`local.InActionSchema`)) "Stop Ability" (`LearningAgentsActions.SpecifyBoolAction` (`local.InActionSchema`)) :!type "Name"))))

(fn `SpecifyAgentObservation`
  (params (InObservationSchema :type "LearningAgentsObservationSchema Object Reference"))
  (returns (OutObservationSchemaElement :type "LearningAgentsObservationSchemaElement Structure"))
  (return (`LearningAgentsObservations.SpecifyStructObservation` (`local.InObservationSchema`) (`|MakeMap` "Boss" (`LearningAgentsObservations.SpecifyStructObservation` (`local.InObservationSchema`) (`|MakeMap` "Location" (`LearningAgentsObservations.SpecifyLocationObservation` (`local.InObservationSchema`)) "Direction" (`LearningAgentsObservations.SpecifyDirectionObservation` (`local.InObservationSchema`)) "Health" (`LearningAgentsObservations.SpecifyFloatObservation` (`local.InObservationSchema`)) "Ability" (`LearningAgentsObservations.SpecifyStructObservation` (`local.InObservationSchema`) (`|MakeMap` "IsUsingAbility1" (`LearningAgentsObservations.SpecifyBoolObservation` (`local.InObservationSchema`)) "IsUsingAbility2" (`LearningAgentsObservations.SpecifyBoolObservation` (`local.InObservationSchema`)) "IsUsingAbility3" (`LearningAgentsObservations.SpecifyBoolObservation` (`local.InObservationSchema`)) "StopUsingAbility" (`LearningAgentsObservations.SpecifyBoolObservation` (`local.InObservationSchema`)) :!type "Name")) :!type "Name")) "HeroAI" (`LearningAgentsObservations.SpecifyStructObservation` (`local.InObservationSchema`) (`|MakeMap` "Location" (`LearningAgentsObservations.SpecifyLocationObservation` (`local.InObservationSchema`)) "Direction" (`LearningAgentsObservations.SpecifyDirectionObservation` (`local.InObservationSchema`)) "Health" (`LearningAgentsObservations.SpecifyFloatObservation` (`local.InObservationSchema`)) "State" (`LearningAgentsObservations.SpecifyStructObservation` (`local.InObservationSchema`) (`|MakeMap` "IsAttacking" (`LearningAgentsObservations.SpecifyBoolObservation` (`local.InObservationSchema`)) "IsBlocking" (`LearningAgentsObservations.SpecifyBoolObservation` (`local.InObservationSchema`)) "IsRolling" (`LearningAgentsObservations.SpecifyBoolObservation` (`local.InObservationSchema`)) :!type "Name")) :!type "Name")) :!type "Name"))))