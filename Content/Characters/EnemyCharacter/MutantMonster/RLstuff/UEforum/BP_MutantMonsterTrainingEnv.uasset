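; Learning Agents training environment that scores, ends and resets episodes for the BP_MutantMonsterRL boss learning to attack a hero.
; Reward pays for melee hits and hero death, penalizes ability spam and use, and clears the one-shot flags it reads.
; Completion reuses that cached state to terminate on excessive distance, either death or getting stuck.
; Reset repositions the boss and respawns the hero AI; older walk-to-hero distance reward logic is left disconnected.
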(fn `GatherAgentCompletion`
  (params (AgentId :type Integer))
  (returns (OutCompletion :type "ELearningAgentsCompletion Enum"))
  (`/Engine/EditorBlueprintResources/StandardMacros.IsValid` (`self.Reward Actor`)
    (:`Is Valid`
      (`/Engine/EditorBlueprintResources/StandardMacros.IsValid` (`self.Nearest Actor`)
        (:`Is Valid`
          (if (> (`KismetMathLibrary.Vector_Distance` (`Actor.K2_GetActorLocation` (`self.Reward Actor`)) (`Actor.K2_GetActorLocation` (`self.Nearest Actor`))) 4000.0)
            (return "Termination")
            (elif (or (`/Game/Characters/EnemyCharacter/MutantMonster/RLstuff/UEforum/BP_MutantMonsterRL.IsDeath` (`self.Reward Actor`)) (`self.Cached Nearest Actor Dead `))
              (return "Termination")
              (elif (`/Game/Characters/EnemyCharacter/MutantMonster/RLstuff/UEforum/BP_MutantMonsterRL.isStucked` (`self.Reward Actor`))
                (return "Termination")
                (else
                  (return "Running"))))))))))

(fn `GatherAgentReward`
  (params (AgentId :type Integer))
  (returns (OutReward :type "Float (single-precision)"))
  (bind _reward_actor (`self.Reward Actor`))
  ; Attacking
  (bind _output_get (set `self.Reward Actor` (`self.GetAgent` AgentId "/Game/Characters/EnemyCharacter/MutantMonster/RLstuff/UEforum/BP_MutantMonsterRL.BP_MutantMonsterRL_C")))
  (set `self.Nearest Actor` (`/Game/Characters/EnemyCharacter/MutantMonster/RLstuff/UEforum/BP_MutantMonsterRL.NearestActor` _output_get))
  (set `self.Cached Melee Hit` (`/Game/Characters/EnemyCharacter/MutantMonster/RLstuff/UEforum/BP_MutantMonsterRL.MeleeHitSuccess` (`self.Reward Actor`)))
  (set `self.Cached Nearest Actor Dead ` (`/Game/Characters/PlayerAI/HeroAI/NormalHeroAI/BP_HeroAICharacter.IsDeath` (`self.Nearest Actor`)))
  (bind _output_get_2 (set `self.Cached ASP` (`/Game/Characters/EnemyCharacter/MutantMonster/RLstuff/UEforum/BP_MutantMonsterRL.AbilitySpamPenalty` (`self.Reward Actor`))))
  (if _output_get_2
    (set `/Game/Characters/EnemyCharacter/MutantMonster/RLstuff/UEforum/BP_MutantMonsterRL.AbilitySpamPenalty` false (`self.Reward Actor`)))
  (if (`self.Cached Melee Hit`)
    (set `/Game/Characters/EnemyCharacter/MutantMonster/RLstuff/UEforum/BP_MutantMonsterRL.MeleeHitSuccess` false (`self.Reward Actor`)))
  (if (`self.Cached Nearest Actor Dead `)
    (set `/Game/Characters/PlayerAI/HeroAI/NormalHeroAI/BP_HeroAICharacter.IsDeath` false (`self.Nearest Actor`)))
  (return (+ (`LearningAgentsRewards.MakeRewardOnCondition` (`self.Cached ASP`) -500.0 "ConditionReward" false null) (`LearningAgentsRewards.MakeRewardOnCondition` (or (`/Game/Characters/EnemyCharacter/MutantMonster/RLstuff/UEforum/BP_MutantMonsterRL.IsUsingAbility1` _reward_actor) (`/Game/Characters/EnemyCharacter/MutantMonster/RLstuff/UEforum/BP_MutantMonsterRL.IsUsingAbility2` _reward_actor) (`/Game/Characters/EnemyCharacter/MutantMonster/RLstuff/UEforum/BP_MutantMonsterRL.IsUsingAbility3` _reward_actor)) -10000.0 "ConditionReward" false null) (`LearningAgentsRewards.MakeRewardOnCondition` (or (not (`KismetSystemLibrary.IsValid` (`self.Nearest Actor`))) (`self.Cached Nearest Actor Dead `)) 100.0 "ConditionReward" false null) (`LearningAgentsRewards.MakeRewardOnCondition` (`self.Cached Melee Hit`) 40.0 "ConditionReward" false null))))

(fn `ResetAgentEpisode`
  (params (AgentId :type Integer))
  (bind _returnvalue (`self.GetAgent` AgentId "/Game/Characters/EnemyCharacter/MutantMonster/RLstuff/UEforum/BP_MutantMonsterRL.BP_MutantMonsterRL_C"))
  (`/Game/Characters/EnemyCharacter/MutantMonster/RLstuff/UEforum/BP_MutantMonsterRL.Boss Reset To Point` _returnvalue)
  (`/Game/Characters/PlayerAI/HeroAI/NormalHeroAI/BP_HeroAICharacter.SpawnHeroAI` (`/Game/Characters/EnemyCharacter/MutantMonster/RLstuff/UEforum/BP_MutantMonsterRL.NearestActor` _returnvalue)))