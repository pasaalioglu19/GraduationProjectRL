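; Mutant monster boss character that registers as a Learning Agents agent for reinforcement learning against hero AI characters.
; Each tick it targets the nearest living hero, fires one of three GAS attacks from a float index, flags repeated picks for a spam penalty and detects being stuck.
; A forward sphere trace reports whether it faces a hero.
; Death triggers a reset that teleports it near the spawn point and restores attributes.
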(event `self.ReceiveBeginPlay`
  ;[1 1 1] Register Agent with Manager
  (`|ExecutionSequence`
    (:`then_0`
      (bind _outactors (`GameplayStatics.GetAllActorsOfClass` "/Game/Characters/PlayerAI/HeroAI/NormalHeroAI/BP_HeroAICharacter.BP_HeroAICharacter_C"))
      (set `self.HeroAI` _outactors))
    (:`then_1`
      (bind _outactors_2 (`GameplayStatics.GetAllActorsWithTag` "LearningAgentsManager"))
      (for _array_element _outactors_2
        (bind _returnvalue (`self.GetComponentByClass` _array_element "/Script/LearningAgents.LearningAgentsManager"))
        (`/Engine/EditorBlueprintResources/StandardMacros.IsValid` _returnvalue
          (:`Is Valid`
            (`LearningAgentsManager.AddAgent` _returnvalue self)
            (set `self.Found Manager` true))))
      (if (not (`self.Found Manager`))
        (`KismetSystemLibrary.PrintString` "Could not find Learning Agents manager. Did we forget to add one to the scene?")))
    (:`then_2`
      (bind _returnvalue_2 (`GameplayStatics.GetActorOfClass` "/Game/Shared/SpawnPoint/BP_SpawnPoint.BP_SpawnPoint_C"))
      (set `self.SpawnLocation` (`self.K2_GetActorLocation` _returnvalue_2)))))

(event `self.ReceiveTick`
  (params (DeltaSeconds :type "Float (single-precision)"))
  (`|ExecutionSequence`
    (:`then_0`
      (`self.Find Nearest Actor to Mutant`))
    (:`then_1`
      (`self.Decide Using Ability`))
    (:`then_2`
      (`self.Fix Stuck Condition`))))

(fn `Boss Reset To Point`
  (`self.K2_SetActorLocation` (`NavigationSystemV1.K2_GetRandomReachablePointInRadius` (`self.SpawnLocation`) 1260.0 null null) false true)
  (`WarriorFunctionLibrary.ResetCharacterAttributes` (`self.WarriorAbilitySystemComponent`))
  (`WarriorFunctionLibrary.RemoveGameplayTagFromActorIfFound` self (struct :`TagName` "Shared.Status.Dead"))
  (set `self.LastActorLocation` (0.0 0.0 0.0))
  (set `self.LastLocationDuration` 0.0)
  (set `self.isStucked` false))

(fn `Decide Using Ability`
  (if (or (`self.IsUsingAbility1`) (`self.IsUsingAbility2`) (`self.IsUsingAbility3`))
    (set `self.LastAbilityTime` 0.0)
    (elif (not (`self.StopUsingAbility`))
      (set `self.CurrentAbilityIndex` (`KismetMathLibrary.FTrunc` (`self.UsingAbilityFloatIndex`)))
      (if (== (`self.LastAbilityIndex`) (`self.CurrentAbilityIndex`))
        (set `self.AbilitySpamPenalty` true)
        (else
          (set `self.AbilitySpamPenalty` false)))
      (switch `int` (`self.CurrentAbilityIndex`)
        (:`0`
          (`WarriorAbilitySystemComponent.TryActivateAbilityByTag` (`self.WarriorAbilitySystemComponent`) (struct :`TagName` "Enemy.Ability.Attack1"))
          (set `self.LastAbilityIndex` 0))
        (:`1`
          (`WarriorAbilitySystemComponent.TryActivateAbilityByTag` (`self.WarriorAbilitySystemComponent`) (struct :`TagName` "Enemy.Ability.Attack2"))
          (set `self.LastAbilityIndex` 1))
        (:`2`
          (`WarriorAbilitySystemComponent.TryActivateAbilityByTag` (`self.WarriorAbilitySystemComponent`) (struct :`TagName` "Enemy.Ability.Attack3"))
          (set `self.LastAbilityIndex` 2))))))

(fn `Find Nearest Actor to Mutant`
  (bind (_distance _returnvalue) (`GameplayStatics.FindNearestActor` (`self.K2_GetActorLocation`) (`self.AliveHeroAI`)))
  (`KismetArrayLibrary.Array_Clear` (`self.AliveHeroAI`))
  (for _array_element (`self.HeroAI`)
    (if (not (`/Game/Characters/PlayerAI/HeroAI/NormalHeroAI/BP_HeroAICharacter.IsDeath` _array_element))
      (`KismetArrayLibrary.Array_Add` (`self.AliveHeroAI`) _array_element)))
  (`/Engine/EditorBlueprintResources/StandardMacros.IsValid` _returnvalue
    (:`Is Valid`
      (bind _asbp_hero_aicharacter (cast `/Game/Characters/PlayerAI/HeroAI/NormalHeroAI/BP_HeroAICharacter` _returnvalue))
      (set `self.NearestActor` _asbp_hero_aicharacter))))

(fn `Fix Stuck Condition`
  (if (`KismetMathLibrary.Vector_IsNearlyZero` (- (`self.LastActorLocation`) (`self.K2_GetActorLocation` self)) 0.01)
    (if (> (`self.LastLocationDuration`) 20.0)
      (set `self.isStucked` true)
      (else
        (set `self.LastLocationDuration` (+ (`self.LastLocationDuration`) (`self.Tick Time`)))))
    (else
      (set `self.LastActorLocation` (`self.K2_GetActorLocation` self))
      (set `self.LastLocationDuration` 0.0))))

(fn `Manage Death`
  (set `self.IsDeath` true)
  (`self.Boss Reset To Point`))

(fn `Trace Rotation`
  (returns (HitHeroActor :type Boolean))
  (bind _returnvalue (`self.K2_GetActorLocation`))
  (set `self.HitHeroActor` false)
  (bind (_outhit _returnvalue_2) (`KismetSystemLibrary.SphereTraceSingle` _returnvalue (+ _returnvalue (* (`self.GetActorForwardVector`) 1000.0)) 180.0 "TraceTypeQuery2"))
  (if _returnvalue_2
    (cast `/Game/Characters/PlayerAI/HeroAI/NormalHeroAI/BP_HeroAICharacter` (`.HitActor` (`GameplayStatics.BreakHitResult` _outhit))
      (:`then`
        (set `self.HitHeroActor` true))
      (:`CastFailed`
        (set `self.HitHeroActor` false)))
    (else
      (set `self.HitHeroActor` false)))
  (return (`self.HitHeroActor`)))

(fn `UserConstructionScript`
  (`parent.UserConstructionScript`))