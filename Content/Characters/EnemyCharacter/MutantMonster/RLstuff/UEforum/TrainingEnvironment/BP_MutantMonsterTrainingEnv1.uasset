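; Learning Agents training environment that trains the MutantMonster RL boss to approach its nearest actor.
; Reward is 2000 minus distance to that actor, with tiered multipliers boosting it at closer range.
; Episodes terminate when the target is very near or too far, checked on actor references cached by the reward function rather than looked up per agent.
; Reset returns the boss to its point and calls SpawnHeroAI on the target.
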(fn `GatherAgentCompletion`
  (params (AgentId :type Integer))
  (returns (OutCompletion :type "ELearningAgentsCompletion Enum"))
  (`/Engine/EditorBlueprintResources/StandardMacros.IsValid` (`self.Reward Actor`)
    (:`Is Valid`
      (`/Engine/EditorBlueprintResources/StandardMacros.IsValid` (`self.Nearest Actor`)
        (:`Is Valid`
          (if (> (`KismetMathLibrary.Vector_Distance` (`Actor.K2_GetActorLocation` (`self.Reward Actor`)) (`Actor.K2_GetActorLocation` (`self.Nearest Actor`))) 4000.0)
            (return "Termination")
            (elif (< (`KismetMathLibrary.Vector_Distance` (`Actor.K2_GetActorLocation` (`self.Reward Actor`)) (`Actor.K2_GetActorLocation` (`self.Nearest Actor`))) 250.0)
              (return "Termination")
              (else
                (return "Running")))))))))

(fn `GatherAgentReward`
  (params (AgentId :type Integer))
  (returns (OutReward :type "Float (single-precision)"))
  (bind _output_get (set `self.Reward Actor` (`self.GetAgent` AgentId "/Game/Characters/EnemyCharacter/MutantMonster/RLstuff/UEforum/BP_MutantMonsterRL.BP_MutantMonsterRL_C")))
  (set `self.Nearest Actor` (`/Game/Characters/EnemyCharacter/MutantMonster/RLstuff/UEforum/BP_MutantMonsterRL.NearestActor` _output_get))
  (set `self.Reward Coef` (- 2000.0 (`Actor.GetDistanceTo` (`self.Reward Actor`) (`self.Nearest Actor`))))
  (if (> (`self.Reward Coef`) 1700.0)
    (set `self.Reward` (* (`self.Reward Coef`) 10.0))
    (elif (> (`self.Reward Coef`) 1600.0)
      (set `self.Reward` (* (`self.Reward Coef`) 7.0))
      (elif (> (`self.Reward Coef`) 1400.0)
        (set `self.Reward` (* (`self.Reward Coef`) 5.0))
        (elif (> (`self.Reward Coef`) 1000.0)
          (set `self.Reward` (* (`self.Reward Coef`) 2.0))
          (elif (> (`self.Reward Coef`) 0.0)
            (set `self.Reward` (`self.Reward Coef`))
            (else
              (set `self.Reward` (`self.Reward Coef`))))))))
  (return (`self.Reward`)))

(fn `ResetAgentEpisode`
  (params (AgentId :type Integer))
  (bind _returnvalue (`self.GetAgent` AgentId "/Game/Characters/EnemyCharacter/MutantMonster/RLstuff/UEforum/BP_MutantMonsterRL.BP_MutantMonsterRL_C"))
  (`/Game/Characters/EnemyCharacter/MutantMonster/RLstuff/UEforum/BP_MutantMonsterRL.Boss Reset To Point` _returnvalue)
  (`/Game/Characters/PlayerAI/HeroAI/NormalHeroAI/BP_HeroAICharacter.SpawnHeroAI` (`/Game/Characters/EnemyCharacter/MutantMonster/RLstuff/UEforum/BP_MutantMonsterRL.NearestActor` _returnvalue)))